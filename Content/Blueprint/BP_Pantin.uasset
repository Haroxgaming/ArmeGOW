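; BP_Pantin is a damageable dummy with a world-space health bar that respawns after its HP runs out.
; Damage events lower HP and update the WBP_health widget, with the fall variant also playing a fall-and-stand-up montage.
; At zero HP it hides mesh and bar, refills HP immediately, then reappears after a delay.
; Every tick, the health bar rotates to face the player camera.
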(event `self.ReceiveBeginPlay`
  (bind _hp_max (`self.HP max`))
  ;[1 1 1] event begin play
  (bind _aswbp_health (cast `/Game/Blueprint/WBP_health` (`WidgetComponent.GetUserWidgetObject` (`self.Health bar`))))
  (bind _output_get (set `self.WBP Heatlh ref` _aswbp_health))
  (bind _output_get_2 (set `self.HP` _hp_max))
  (`/Game/Blueprint/WBP_health.Update health` _output_get _output_get_2 _hp_max))

(event `self.ReceiveTick`
  (params (DeltaSeconds :type "Float (single-precision)"))
  ;[1 1 1] Widget rotate
  (`SceneComponent.K2_SetWorldRotation` (`self.Health bar`) (`KismetMathLibrary.FindLookAtRotation` (`SceneComponent.K2_GetComponentLocation` (`self.Health bar`)) (`self.K2_GetActorLocation` (`PlayerController.PlayerCameraManager` (`GameplayStatics.GetPlayerController` 0)))) false false))

(event `take damage`
  (params (Damage :type "Float (double-precision)"))
  ;[1 1 1] Take damage
  (set `self.HP` (- (`self.HP`) Damage))
  (`/Game/Blueprint/WBP_health.Update health` (`self.WBP Heatlh ref`) (`self.HP`) (`self.HP max`) :!label _label)
  (if (<= (`self.HP`) 0.0)
    (`self.respawn`)))

(event `fall`
  (params (Damage :type "Float (double-precision)"))
  ;[1 1 1] fall
  (`|PlayMontage` (`self.SkeletalMesh`) "/Game/Animation/AM_FallAndStandUp.AM_FallAndStandUp"
    (:`then`
      (set `self.HP` (- (`self.HP`) Damage))
      (goto _label))))

(event `respawn`
  (bind _hp_max (`self.HP max`))
  ;[1 1 1] Respawn
  (`SceneComponent.SetVisibility` (`self.SkeletalMesh`) false false)
  (`SceneComponent.SetVisibility` (`self.Health bar`) false false)
  (bind _output_get (set `self.HP` _hp_max))
  (`/Game/Blueprint/WBP_health.Update health` (`self.WBP Heatlh ref`) _output_get _hp_max)
  (`KismetSystemLibrary.Delay` 8.0)
  (`SceneComponent.SetVisibility` (`self.SkeletalMesh`) true false)
  (`SceneComponent.SetVisibility` (`self.Health bar`) true false))

(fn `UserConstructionScript`)