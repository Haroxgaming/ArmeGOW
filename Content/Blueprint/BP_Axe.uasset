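; BP_Axe is a short-lived axe attack actor that damages BP_Pantin targets.
; On BeginPlay it caches the player character, and a Rotate timeline drives its pitch, with a DoOnce starting a delayed self-destruct.
; Any box overlap destroys it, calling TakeDamage first if the other actor is a BP_Pantin.
; Both the overlap and timeout paths set the player's CanAttack to false.
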(event `self.ReceiveBeginPlay`
  (bind (_returnvalue_roll _returnvalue_pitch _returnvalue_yaw) (`KismetMathLibrary.BreakRotator` (`self.K2_GetActorRotation`)))
  (bind _returnvalue (`GameplayStatics.GetActorOfClass` "/Game/ThirdPerson/Blueprints/BP_ThirdPersonCharacter.BP_ThirdPersonCharacter_C"))
  (set `self.Player ref` _returnvalue)
  (bind (_direction _rotate) (`Timeline|Rotate` :!via `PlayFromStart`)
    (:`Update`
      (`self.K2_SetActorRotation` (`KismetMathLibrary.MakeRotator` _returnvalue_roll (* (.y _rotate) 3.0) _returnvalue_yaw))
      (`/Engine/EditorBlueprintResources/StandardMacros.DoOnce` false
        (:`Completed`
          (`KismetSystemLibrary.Delay` 1.5)
          (set `/Game/ThirdPerson/Blueprints/BP_ThirdPersonCharacter.Can Attack` false (`self.Player ref`))
          (`self.K2_DestroyActor`))))))

(event `self.Box.OnComponentBeginOverlap`
  (params (OverlappedComponent :type "PrimitiveComponent Object Reference") (OtherActor :type "Actor Object Reference") (OtherComp :type "PrimitiveComponent Object Reference") (OtherBodyIndex :type Integer) (bFromSweep :type Boolean) (SweepResult :type "HitResult Structure (by ref)"))
  (set `/Game/ThirdPerson/Blueprints/BP_ThirdPersonCharacter.Can Attack` false (`self.Player ref`))
  (bind _asbp_pantin (cast `/Game/Blueprint/BP_Pantin` OtherActor)
    (:`then`
      (`/Game/Blueprint/BP_Pantin.take damage` _asbp_pantin (`self.Damage`))
      (`self.K2_DestroyActor`))
    (:`CastFailed`
      (`self.K2_DestroyActor`))))

(fn `UserConstructionScript`)